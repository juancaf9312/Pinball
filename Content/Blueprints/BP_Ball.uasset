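; BP_Ball is a pinball ball actor that plays an attached "ball added" sound when it spawns.
; Each tick it applies a constant DefaultSpeed impulse as acceleration, plus a pull into the surface found by a downward line trace, scaled by TableStickyness along the inverted impact normal to keep it on the table.
; Velocity magnitude drives the clamped volume and pitch of the rolling sound.
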(event `self.ReceiveBeginPlay`
  (`GameplayStatics.SpawnSoundAttached` "/Game/Assets/Sounds/Pinball_BallAdded_Cue.Pinball_BallAdded_Cue" (`self.Ball`)))

(event `self.ReceiveTick`
  (params (DeltaSeconds :type "Float (single-precision)"))
  (bind _returnvalue (`self.K2_GetActorLocation`))
  (bind _ballrollingsound (`self.BallRollingSound`))
  (bind _returnvalue_2 (/ (`KismetMathLibrary.VSize` (`self.GetVelocity`)) 1000.0))
  (`|ExecutionSequence`
    (:`then_0`
      (`PrimitiveComponent.AddImpulse` (`self.Ball`) (* (`self.DefaultSpeed`) DeltaSeconds) "None" true)
      (bind _outhit (`KismetSystemLibrary.LineTraceSingle` _returnvalue (- _returnvalue (0.0 0.0 500.0)) "TraceTypeQuery1"))
      (`PrimitiveComponent.AddImpulse` (`self.Ball`) (* (* (`.ImpactNormal` (`GameplayStatics.BreakHitResult` _outhit)) -1.0) (* (`self.TableStickyness`) DeltaSeconds)) "None" true))
    (:`then_1`
      (`AudioComponent.SetVolumeMultiplier` _ballrollingsound (`KismetMathLibrary.FClamp` _returnvalue_2))
      (`AudioComponent.SetPitchMultiplier` _ballrollingsound (`KismetMathLibrary.FClamp` _returnvalue_2 0.97 1.2)))))

(fn `UserConstructionScript`)