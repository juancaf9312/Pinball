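; BP_DropTarget is a pinball drop target that shows a configurable letter, set on its text render in the construction script.
; On a hit it slides its mesh down, disables collision, plays a bell sound and fires the OnDrop dispatcher.
; ResetTarget raises the mesh and restores collision.
; At BeginPlay it binds an event to the pinball game mode's OnGameReset dispatcher.
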(event `self.ReceiveBeginPlay`
  (bind _aspinball_game_mode (cast `/Game/Blueprints/PinballGameMode` (`GameplayStatics.GetGameMode`)))
  (add `/Game/Blueprints/PinballGameMode.OnGameReset` _aspinball_game_mode (`|CreateDelegate` :!event `ResetTarget`)))

(event `Drop`
  (`KismetSystemLibrary.MoveComponentTo` (`self.DTMesh`) (0.0 0.0 -110.0))
  (`PrimitiveComponent.SetCollisionEnabled` (`self.DTMesh`) "NoCollision")
  (`GameplayStatics.PlaySoundAtLocation` "/Game/Assets/Sounds/Pinball_Bell01_Cue.Pinball_Bell01_Cue" (`self.K2_GetActorLocation`)))

(event `ResetTarget`
  (`KismetSystemLibrary.MoveComponentTo` (`self.DTMesh`) (0.0 0.0 0.0))
  (`PrimitiveComponent.SetCollisionEnabled` (`self.DTMesh`) "QueryAndPhysics"))

(event `self.ReceiveHit`
  (params (MyComp :type "PrimitiveComponent Object Reference") (Other :type "Actor Object Reference") (OtherComp :type "PrimitiveComponent Object Reference") (bSelfMoved :type Boolean) (HitLocation :type "Vector Structure") (HitNormal :type "Vector Structure") (NormalImpulse :type "Vector Structure") (Hit :type "HitResult Structure (by ref)"))
  (`self.Drop`)
  (`self.OnDrop`))

(fn `UserConstructionScript`
  (`TextRenderComponent.K2_SetText` (`self.TextRender`) (`KismetTextLibrary.Conv_StringToText` (`self.DropLetter`))))